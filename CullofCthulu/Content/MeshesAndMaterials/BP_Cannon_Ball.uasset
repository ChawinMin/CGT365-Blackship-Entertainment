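; BP_Cannon_Ball is a cannon projectile that damages BP_Serpent actors it overlaps.
; The hitbox's begin overlap passes through a DoOnce, reset on end overlap, into DamageToSerpent with the regular damage value.
; That function subtracts the damage from the serpent's health, destroys the serpent at zero or below, plays a hit sound and removes the ball's Sphere component, leaving the actor itself alive.
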(event `self.Cannon Hitbox.OnComponentBeginOverlap`
  (params (OverlappedComponent :type "PrimitiveComponent Object Reference") (OtherActor :type "Actor Object Reference") (OtherComp :type "PrimitiveComponent Object Reference") (OtherBodyIndex :type Integer) (bFromSweep :type Boolean) (SweepResult :type "HitResult Structure (by ref)"))
  ; Detect if the Serpent collides with the cannon ball
  (`/Engine/EditorBlueprintResources/StandardMacros.DoOnce` false :!label _label
    (:`Completed`
      (`self.DamageToSerpent` OtherActor (`self.Regular Damage`)))))

(event `self.Cannon Hitbox.OnComponentEndOverlap`
  (params (OverlappedComponent :type "PrimitiveComponent Object Reference") (OtherActor :type "Actor Object Reference") (OtherComp :type "PrimitiveComponent Object Reference") (OtherBodyIndex :type Integer))
  ; Detect if the Serpent collides with the cannon ball
  (goto _label :!via `Reset`))

(fn `DamageToSerpent`
  (params (`Other Actor` :type "Actor Object Reference") (Damage :type "Float (double-precision)"))
  (bind _sphere (`self.Sphere`))
  ; Deal damage to the serpent and check if it's health fall below a threshold
  (bind _asbp_serpent (cast `/Game/ThirdPerson/Blueprints/Enemies/BP_Serpent` `Other Actor`))
  (bind _output_get (set `self.Cannon Ball Damage` Damage))
  (set `/Game/ThirdPerson/Blueprints/Enemies/BP_Serpent.SerpentHealth` (- (`/Game/ThirdPerson/Blueprints/Enemies/BP_Serpent.SerpentHealth` _asbp_serpent) _output_get) _asbp_serpent)
  (if (<= (`/Game/ThirdPerson/Blueprints/Enemies/BP_Serpent.SerpentHealth` _asbp_serpent) 0.0)
    (`self.K2_DestroyActor` _asbp_serpent))
  (`GameplayStatics.PlaySound2D` "/Game/Assets/Sounds_CoCthulu/Others/Enemies/Damaged/Sfx_SoftSkin_Damaged.Sfx_SoftSkin_Damaged" 1.0 1.0 0.0 null null)
  (if (`KismetSystemLibrary.IsValid` _sphere)
    (`ActorComponent.K2_DestroyComponent` _sphere)))

(fn `UserConstructionScript`)