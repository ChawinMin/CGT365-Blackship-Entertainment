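; Enemy cannon ball actor that damages the ship it hits.
; On overlap with a BP_Ship, it calls the ship's DamageToShip with a fixed damage amount and impact sound, then destroys itself.
; DamageToPlayer has an empty body; its serpent health, sound and sphere removal logic is disconnected and never runs.
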(event `self.ReceiveActorBeginOverlap`
  (params (OtherActor :type "Actor Object Reference"))
  (bind _asbp_ship (cast `/Game/ThirdPerson/Blueprints/BP_Ship` OtherActor))
  (`/Game/ThirdPerson/Blueprints/BP_Ship.DamageToShip` _asbp_ship "/Game/Assets/Sounds_CoCthulu/Ship/Sfx_Ship_Damaged_WithWaveCrash.Sfx_Ship_Damaged_WithWaveCrash" 50.0)
  (`self.K2_DestroyActor`))

(fn `DamageToPlayer`
  (params (`Other Actor` :type "Actor Object Reference") (Damage :type "Float (double-precision)"))
  ; Deal damage to the serpent and check if it's health fall below a threshold
)

(fn `UserConstructionScript`)