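; BP_Tower is a hostile turret that lobs cannonballs at the player's ship while it is in range.
; Range overlaps drive a delayed firing loop, with an Attacking flag preventing duplicate loops.
; Each shot yaws toward the player and computes ballistic pitch from horizontal distance, assuming fixed speed and gravity and ignoring height difference.
; Player cannonballs hitting the Hitbox reduce Health; destroying the tower heals the ship, capped at its maximum.
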(event `self.Hitbox.OnComponentBeginOverlap`
  (params (OverlappedComponent :type "PrimitiveComponent Object Reference") (OtherActor :type "Actor Object Reference") (OtherComp :type "PrimitiveComponent Object Reference") (OtherBodyIndex :type Integer) (bFromSweep :type Boolean) (SweepResult :type "HitResult Structure (by ref)"))
  ; Damaged by player
  (bind _asbp_base_cannon_ball (cast `/Game/ThirdPerson/Blueprints/Cannon/BP_Base_Cannon_Ball` OtherActor))
  ;; Damage Tower
  (bind _output_get (set `self.Health` (- (`self.Health`) (`/Game/ThirdPerson/Blueprints/Cannon/BP_Base_Cannon_Ball.Regular Damage` _asbp_base_cannon_ball))))
  (`self.K2_DestroyActor` _asbp_base_cannon_ball)
  ;; Check if Dead
  (if (<= _output_get 0.0)
    ;; If dead, heal and destroy tower
    (`GameplayStatics.PlaySound2D` "/Game/Assets/Sounds_CoCthulu/Towers/Sfx_Tower_Damaged.Sfx_Tower_Damaged" 1.0 1.0 0.0 null null)
    (bind _asbp_ship (cast `/Game/ThirdPerson/Blueprints/BP_Ship` (`GameplayStatics.GetPlayerCharacter` 0)))
    (bind _returnvalue (+ (`/Game/ThirdPerson/Blueprints/BP_Ship.Ship Health` _asbp_ship) 50))
    (bind _max_ship_health (`/Game/ThirdPerson/Blueprints/BP_Ship.Max Ship Health` _asbp_ship))
    (if (<= _returnvalue _max_ship_health)
      (set `/Game/ThirdPerson/Blueprints/BP_Ship.Ship Health` _returnvalue _asbp_ship)
      (else
        (set `/Game/ThirdPerson/Blueprints/BP_Ship.Ship Health` (`KismetMathLibrary.FTrunc` _max_ship_health) _asbp_ship)))
    (`self.K2_DestroyActor`)
    (else
      ;; If alive, play sound
      (`GameplayStatics.PlaySound2D` "/Game/Assets/Sounds_CoCthulu/Towers/Sfx_Tower_Damaged.Sfx_Tower_Damaged" 1.0 1.0 0.0 null null))))

(event `self.Range.OnComponentEndOverlap`
  (params (OverlappedComponent :type "PrimitiveComponent Object Reference") (OtherActor :type "Actor Object Reference") (OtherComp :type "PrimitiveComponent Object Reference") (OtherBodyIndex :type Integer))
  ; Stop Attacking Player if Outside Range
  (cast `/Game/ThirdPerson/Blueprints/BP_Ship` OtherActor)
  (set `self.PlayerInRange?` false))

(event `self.Range.OnComponentBeginOverlap`
  (params (OverlappedComponent :type "PrimitiveComponent Object Reference") (OtherActor :type "Actor Object Reference") (OtherComp :type "PrimitiveComponent Object Reference") (OtherBodyIndex :type Integer) (bFromSweep :type Boolean) (SweepResult :type "HitResult Structure (by ref)"))
  (bind _returnvalue (`GameplayStatics.GetPlayerCharacter` 0))
  (bind _cannonarrow (`self.CannonArrow`))
  (bind (_returnvalue_x _returnvalue_y) (`KismetMathLibrary.BreakVector` (`self.K2_GetActorLocation` _returnvalue)))
  (bind (_returnvalue_x_2 _returnvalue_y_2) (`KismetMathLibrary.BreakVector` (`self.K2_GetActorLocation` (`ActorComponent.GetOwner` (`self.CannonArrow`)))))
  (cast `/Game/ThirdPerson/Blueprints/BP_Ship` OtherActor)
  ; Checks if player is in activatable range (not hitting range) and if it already is attacking
  (set `self.PlayerInRange?` true)
  (if (not (`self.Attacking?`))
    (set `self.Attacking?` true)
    (`/Game/ThirdPerson/Blueprints/DelayLoopMacros.WhileLoopWithDelay` (`self.PlayerInRange?`) 5.0
      (:`LoopBody`
        ; Shooting code
        (`SceneComponent.K2_SetWorldRotation` (`self.CannonArrow`) (`KismetMathLibrary.MakeRotator` 0.0 (/ (`KismetMathLibrary.DegAsin` (/ (* (`KismetMathLibrary.Sqrt` (+ (`KismetMathLibrary.Square` (- _returnvalue_y _returnvalue_y_2)) (`KismetMathLibrary.Square` (- _returnvalue_x _returnvalue_x_2)))) 980.0) (`KismetMathLibrary.Square` 1500.0))) 2.0) (.yaw (`KismetMathLibrary.FindLookAtRotation` (`SceneComponent.K2_GetComponentLocation` (`self.DefaultSceneRoot`)) (`self.K2_GetActorLocation` _returnvalue)))) false false)
        (`GameplayStatics.SpawnSound2D` "/Game/Assets/Sounds_CoCthulu/Cannons/Sfx_EnemyCannonFire.Sfx_EnemyCannonFire" 1.0 1.0 0.0 null)
        (`GameplayStatics.SpawnEmitterAtLocation` "/Game/StarterContent/Particles/P_Explosion.P_Explosion" (`SceneComponent.GetSocketLocation` _cannonarrow "None"))
        (`|SpawnActorFromClass` "/Game/ThirdPerson/Blueprints/Enemies/BP_Tower_Cannon_Ball.BP_Tower_Cannon_Ball_C" (`SceneComponent.K2_GetComponentToWorld` _cannonarrow) "Undefined" "MultiplyWithRoot" null 0.0 null))
      (:`Completed`
        (set `self.Attacking?` false)))))

(fn `UserConstructionScript`)